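; BP_MasterTile is a track tile for an endless spaceship runner that spawns collectible orbs and chains the next tile.
; On BeginPlay in a specific game state, it may add an orb child actor above one of three random lanes, using a random material from SpaceshipGameMode.
; When BP_Spaceship overlaps SpawnTrigger, it asks the game mode to spawn another tile, then destroys itself after a delay.
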(event OnComponentBeginOverlap(SpawnTrigger)
  (params (OverlappedComponent :type Primitive%20Component%20Object%20Reference) (OtherActor :type Actor%20Object%20Reference) (OtherComp :type Primitive%20Component%20Object%20Reference) (OtherBodyIndex :type Integer) (bFromSweep :type Boolean) (SweepResult :type Hit%20Result%20Structure%20%28by%20ref%29))
  ;[1 1 1] Spawn New Tile
  (Utilities|Casting|CastToBP_Spaceship OtherActor)
  (bind _asspaceship_game_mode (Utilities|Casting|CastToSpaceshipGameMode (Game|GetGameMode)))
  (Default|SpawnTile _asspaceship_game_mode)
  (Utilities|FlowControl|Delay 12.0)
  (Actor|DestroyActor))

(event EventBeginPlay
  ;[1 1 1] Spawn Orbs
  (bind _asspaceship_game_mode (Utilities|Casting|CastToSpaceshipGameMode (Game|GetGameMode)))
  (if (Utilities|Enum|Equal(Enum) (Variables|/Game/_Game/Blueprints/GameModes/SpaceshipGameMode.SpaceshipGameMode_C|GetStateOfTheGame _asspaceship_game_mode) "NewEnumerator2")
    (CallFunction|SpawnOrbs)))

(fn ConstructionScript)

(fn SpawnOrbs
  (if (Math|Float|InRange(Float) (Math|Random|RandomFloatinRange 0.0 1.0) 0.0 (Variables|Default|GetOrbSpawnRate))
    (switch int (Math|Random|RandomIntegerinRange 0 2)
      (:Default
        (Variables|Default|SetOrbLane (Variables|Default|GetLane1) :!label _label))
      (:0
        (Variables|Default|SetOrbLane (Variables|Default|GetLane0)))
      (:1
        (goto _label))
      (:2
        (Variables|Default|SetOrbLane (Variables|Default|GetLane2))))
    (bind _returnvalue (AddComponent|AddChildActorComponent false (Math|Transform|MakeTransform (Math|Vector|MakeVector (.x (.location (Transformation|GetRelativeTransform (Variables|Default|GetOrbLane)))) (.y (.location (Transformation|GetRelativeTransform (Variables|Default|GetOrbLane)))) (+ (.z (.location (Transformation|GetRelativeTransform (Variables|Default|GetOrbLane)))) 1.5e+02)) (.rotation (Transformation|GetRelativeTransform (Variables|Default|GetOrbLane))) (.scale (Transformation|GetRelativeTransform (Variables|Default|GetOrbLane))))))
    (bind _asbp_orb (Utilities|Casting|CastToBP_Orb (Variables|/Script/Engine.ChildActorComponent|GetChildActor _returnvalue)))
    (CallFunction|SetRandomCollectibleMaterial _asbp_orb)))

(fn SetRandomCollectibleMaterial
  (params (Orb :type BP%20Orb%20Object%20Reference))
  (bind _asspaceship_game_mode (Utilities|Casting|CastToSpaceshipGameMode (Game|GetGameMode)))
  (Rendering|Material|SetMaterial (Variables|/Game/_Game/Blueprints/BP_Orb.BP_Orb_C|GetStaticMesh Orb) 0 (.OutItem (Utilities|Array|Random (Variables|/Game/_Game/Blueprints/GameModes/SpaceshipGameMode.SpaceshipGameMode_C|GetCollectibleMaterials _asspaceship_game_mode)))))