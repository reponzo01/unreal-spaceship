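; Game mode for a spaceship game that builds the starting track, runs the game-state flow and picks collectible instructions.
; BeginPlay sets Ready, then chains first and master tiles, each spawned at the previous tile's SpawnPoint.
; SetGameState switches input mode and fires instruction or play calls, while Tick counts down during Instructions before entering Playing.
; A random instruction is chosen from options filtered by the game instance's collected materials, and the preview mesh is shown glowing blue.
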(event Custom|SetGameState
  (params (GameState :type StateOfGame%20Enum :default "NewEnumerator0"))
  ;[1 1 1] Set Game State
  (switch Utilities|FlowControl|Switch|SwitchonStateOfGame GameState
    (:NewEnumerator3
      ;;[0.9456 1 0] Ready
      (Variables|Default|SetStateOfTheGame "NewEnumerator3"))
    (:NewEnumerator0
      ;;[0 0.9275 1] Instructions
      (Variables|Default|SetStateOfTheGame "NewEnumerator0")
      (Input|SetInputModeUIOnly (Game|GetPlayerController 0) 0 "DoNotLock")
      (Variables|Default|SetCountdown (Variables|Default|GetCountdownMaxSeconds))
      (Default|CallShowInstructionsCollectible))
    (:NewEnumerator1
      ;;[1 0 0] Countdown (may not need)
      (Variables|Default|SetCountdown (Variables|Default|GetCountdownMaxSeconds))
      (Variables|Default|SetStateOfTheGame "NewEnumerator1"))
    (:NewEnumerator2
      ;;[0 1 0.1645] Playing
      (Default|CallStartPlaying)
      (Variables|Default|SetStateOfTheGame "NewEnumerator2")
      (Input|SetInputModeGameandUI (Game|GetPlayerController 0) 0 "LockAlways" false))))

(event EventBeginPlay
  ;[1 1 1] Begin Play
  (CallFunction|SetGameState "NewEnumerator3")
  (Utilities|FlowControl|Sequence
    (:then_0
      (for _index (range 0 2)
        (CallFunction|SpawnFirstTile)))
    (:then_1
      (for _index_2 (range 0 9)
        (CallFunction|SpawnTile)))))

(event EventTick
  (params (DeltaSeconds :type Float%20%28single-precision%29))
  ;[1 1 1] Countdown
  (if (Utilities|Enum|Equal(Enum) (Variables|Default|GetStateOfTheGame) "NewEnumerator0")
    (bind _output_get (Variables|Default|SetCountdown (- (Variables|Default|GetCountdown) DeltaSeconds)))
    (if (>= _output_get 2.0)
      (Variables|Default|SetCount 3)
      (elif (>= _output_get 1.0)
        (Variables|Default|SetCount 2)
        (elif (>= _output_get 0.0)
          (Variables|Default|SetCount 1)
          (else
            (CallFunction|SetGameState "NewEnumerator2")))))))

(fn ConstructionScript)

(fn SpawnTile
  (bind _returnvalue (Game|SpawnActorfromClass "/Game/_Game/Blueprints/BP_MasterTile.BP_MasterTile_C" (Variables|Default|GetNextSpawnPoint) "Undefined" 0 0))
  (Variables|Default|SetNextSpawnPoint (Math|Transform|MakeTransform (Transformation|GetWorldLocation (Variables|/Game/_Game/Blueprints/BP_MasterTile.BP_MasterTile_C|GetSpawnPoint _returnvalue)) "0, 0, 0" "1,1,1")))

(fn SpawnFirstTile
  (bind _returnvalue (Game|SpawnActorfromClass "/Game/_Game/Blueprints/BP_FirstTile.BP_FirstTile_C" (Variables|Default|GetNextSpawnPoint) "Undefined" 0 0))
  (Variables|Default|SetNextSpawnPoint (Math|Transform|MakeTransform (Transformation|GetWorldLocation (Variables|/Game/_Game/Blueprints/BP_FirstTile.BP_FirstTile_C|GetSpawnPoint _returnvalue)) "0, 0, 0" "1,1,1")))

(fn ShowInstructionsforRandomCollectible
  (params (InstructionsCollectibleMesh :type Static%20Mesh%20Component%20Object%20Reference))
  (bind _availableinstructions (Variables|Default|GetAvailableInstructions))
  (bind _availableinstructions_2 (Variables|Default|GetAvailableInstructions))
  (bind _availableinstructions_3 (Variables|Default|GetAvailableInstructions))
  (Variables|Default|GetRefToSpaceshipGameInstance
    (:then
      (Variables|Default|SetRefToCurrentCollectibleMaterials (Variables|/Game/_Game/Blueprints/GameModes/SpaceshipGameInstance.SpaceshipGameInstance_C|GetCurrentCollectibleMaterials (Variables|Default|GetRefToSpaceshipGameInstance)) :!label _label)
      (Utilities|Array|Clear (Variables|Default|GetAvailableInstructions))
      (if (<= (Utilities|Set|Length (Variables|Default|GetRefToCurrentCollectibleMaterials)) 0) ; Current Collectible Set is Empty
        (Utilities|Array|Add _availableinstructions "NewEnumerator0")
        (Utilities|Array|Add _availableinstructions "NewEnumerator2")
        (elif (== (Utilities|Set|Length (Variables|Default|GetRefToCurrentCollectibleMaterials)) (Utilities|Array|Length (Variables|Default|GetCollectibleMaterials))) ; Collectible Materials Set is Full
          (Utilities|Array|Add _availableinstructions_2 "NewEnumerator1")
          (Utilities|Array|Add _availableinstructions_2 "NewEnumerator2")
          (else
            (Utilities|Array|Add _availableinstructions_3 "NewEnumerator0")
            (Utilities|Array|Add _availableinstructions_3 "NewEnumerator1")
            (Utilities|Array|Add _availableinstructions_3 "NewEnumerator2"))))
      (Variables|Default|SetCurrentInstruction (.OutItem (Utilities|Array|Random (Variables|Default|GetAvailableInstructions))))
      (Utilities|IsValid InstructionsCollectibleMesh
        (:Is%20Valid
          (Rendering|Material|SetMaterial InstructionsCollectibleMesh 0 "/Game/_Game/Materials/MI_GlowBlue.MI_GlowBlue")
          (Rendering|SetVisibility InstructionsCollectibleMesh true false))))
    (:else
      (bind _asspaceship_game_instance (Utilities|Casting|CastToSpaceshipGameInstance (Game|GetGameInstance))
        (:then
          (Variables|Default|SetRefToSpaceshipGameInstance _asspaceship_game_instance)
          (goto _label))
        (:CastFailed
          (Development|PrintString "fail"))))))