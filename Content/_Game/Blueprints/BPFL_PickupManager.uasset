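; Blueprint function library that expires timed pickups in the spaceship game.
; ManagePickupDeactivation walks a snapshot of the keys in the game instance's CurrentPickups map and compares elapsed game time since each pickup's start with its duration.
; Expired entries are removed from the map, and the game mode broadcasts a pickup-removed event for each one.
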(fn ManagePickupDeactivation
  (params (SpaceshipGameInstance :type Spaceship%20Game%20Instance%20Object%20Reference%20%28by%20ref%29) (SpaceshipGameMode :type Spaceship%20Game%20Mode%20Object%20Reference))
  (bind _currentpickups (Variables|/Game/_Game/Blueprints/GameModes/SpaceshipGameInstance.SpaceshipGameInstance_C|GetCurrentPickups SpaceshipGameInstance))
  ;[1 0 0] Careful here. Removing elements within a loop. May have to iterate backwards. Find a way to test.
  (if (> (Utilities|Map|Length _currentpickups) 0)
    (bind _keys (Utilities|Map|Keys _currentpickups))
    (for _array_element _keys
      (if (.ReturnValue (Utilities|Map|Find _currentpickups _array_element))
        (if (> (- (Utilities|Time|GetTimeSeconds) (.PickupStartTime (Utilities|Struct|BreakST_Pickup (.Value (Utilities|Map|Find _currentpickups _array_element))))) (.PickupDuration (Utilities|Struct|BreakST_Pickup (.Value (Utilities|Map|Find _currentpickups _array_element)))))
          (Utilities|Map|Remove _currentpickups _array_element)
          (Default|EventBroadcastPickupRemoved SpaceshipGameMode _array_element))))))