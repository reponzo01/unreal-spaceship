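; Collectible orb that awards score through SpaceshipGameMode and destroys itself when picked up.
; On overlap with BP_Spaceship, it scores only if its material is among the game instance's current collectible materials.
; Game mode pickup events toggle Free for All, which swaps the orb mesh for the pickup mesh and lets any overlap score, skipping the spaceship and material checks.
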(event OnComponentBeginOverlap(OrbMesh)
  (params (OverlappedComponent :type Primitive%20Component%20Object%20Reference) (OtherActor :type Actor%20Object%20Reference) (OtherComp :type Primitive%20Component%20Object%20Reference) (OtherBodyIndex :type Integer) (bFromSweep :type Boolean) (SweepResult :type Hit%20Result%20Structure%20%28by%20ref%29))
  (if (Variables|Default|GetAlwaysAwardScore)
    ;[1 1 1] Award Score
    (bind _asspaceship_game_mode (Utilities|Casting|CastToSpaceshipGameMode (Game|GetGameMode) :!label _label))
    (Default|AwardScore _asspaceship_game_mode)
    (Actor|DestroyActor)
    (else
      ;[1 1 1] Check if currently collecting
      (Utilities|Casting|CastToBP_Spaceship OtherActor)
      (CallFunction|SetValidSpaceshipGameInstance)
      (bind _asmaterial_instance (Utilities|Casting|CastToMaterialInstance (Rendering|Material|GetMaterial (Variables|Default|GetOrbMesh) 0)))
      (if (Utilities|Set|Contains (Variables|/Game/_Game/Blueprints/GameModes/SpaceshipGameInstance.SpaceshipGameInstance_C|GetCurrentCollectibleMaterials (Variables|Default|GetRefToSpaceshipGameInstance)) _asmaterial_instance)
        (goto _label)))))

(event EventBeginPlay
  (CallFunction|SetValidSpaceshipGameMode)
  (|BindCustomEvents))

(fn ConstructionScript)

(fn HandlePickupCollected
  (params (PickupType :type PickupType%20Enum :default "NewEnumerator0"))
  (switch Utilities|FlowControl|Switch|SwitchonPickupType PickupType
    (:NewEnumerator0
      ;[1 1 1] Free For All Pickup
      (Variables|Default|SetAlwaysAwardScore true)
      (Utilities|FlowControl|Sequence
        (:then_0
          (bind _pickupmesh (Variables|Default|GetPickupMesh)
            (:then
              (Rendering|SetVisibility _pickupmesh true false))
            (:else)))
        (:then_1
          (bind _orbmesh (Variables|Default|GetOrbMesh)
            (:then
              (Rendering|SetVisibility _orbmesh false false))
            (:else)))))))

(fn HandlePickupRemoved
  (params (PickupType :type PickupType%20Enum :default "NewEnumerator0"))
  (switch Utilities|FlowControl|Switch|SwitchonPickupType PickupType
    (:NewEnumerator0
      ;[1 1 1] Free For All Pickup
      (Variables|Default|SetAlwaysAwardScore false)
      (Utilities|FlowControl|Sequence
        (:then_0
          (bind _pickupmesh (Variables|Default|GetPickupMesh)
            (:then
              (Rendering|SetVisibility _pickupmesh false false))
            (:else)))
        (:then_1
          (bind _orbmesh (Variables|Default|GetOrbMesh)
            (:then
              (Rendering|SetVisibility _orbmesh true false))
            (:else)))))))

(fn SetValidSpaceshipGameMode
  (Variables|Default|GetRefToSpaceshipGameMode
    (:then)
    (:else
      (bind _asspaceship_game_mode (Utilities|Casting|CastToSpaceshipGameMode (Game|GetGameMode)))
      (Variables|Default|SetRefToSpaceshipGameMode _asspaceship_game_mode))))

(fn SetValidSpaceshipGameInstance
  (Variables|Default|GetRefToSpaceshipGameInstance
    (:then)
    (:else
      (bind _asspaceship_game_instance (Utilities|Casting|CastToSpaceshipGameInstance (Game|GetGameInstance)))
      (Variables|Default|SetRefToSpaceshipGameInstance _asspaceship_game_instance))))

(event Custom|EventPickupCollected
  (params (PickupType :type PickupType%20Enum :default "NewEnumerator0"))
  (CallFunction|HandlePickupCollected PickupType))

(event Custom|EventPickupRemoved
  (params (PickupType :type PickupType%20Enum :default "NewEnumerator0"))
  (CallFunction|HandlePickupRemoved PickupType))