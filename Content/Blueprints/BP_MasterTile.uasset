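; BP_MasterTile is a track tile for an endlessly spawned, three-lane spaceship course.
; On BeginPlay, SpawnOrbs adds a child actor component above each lane, using that lane's relative transform raised along Z.
; When BP_Spaceship overlaps SpawnTrigger, the tile asks StarshipGameMode to spawn another tile, then destroys itself after a delay.
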(event OnComponentBeginOverlap(SpawnTrigger)
  (params (OverlappedComponent :type Primitive%20Component%20Object%20Reference) (OtherActor :type Actor%20Object%20Reference) (OtherComp :type Primitive%20Component%20Object%20Reference) (OtherBodyIndex :type Integer) (bFromSweep :type Boolean) (SweepResult :type Hit%20Result%20Structure%20%28by%20ref%29))
  (Utilities|Casting|CastToBP_Spaceship OtherActor)
  (bind _asstarship_game_mode (Utilities|Casting|CastToStarshipGameMode (Game|GetGameMode)))
  (Default|SpawnTile _asstarship_game_mode)
  (Utilities|FlowControl|Delay 12.0)
  (Actor|DestroyActor))

(event EventBeginPlay
  (CallFunction|SpawnOrbs))

(fn ConstructionScript)

(fn SpawnOrbs
  (bind _lane0 (Variables|Default|GetLane0))
  (bind _lane1 (Variables|Default|GetLane1))
  (bind _lane2 (Variables|Default|GetLane2))
  (bind _returnvalue (Transformation|GetRelativeTransform _lane2))
  (bind _returnvalue_2 (Transformation|GetRelativeTransform _lane1))
  (bind _returnvalue_3 (Transformation|GetRelativeTransform _lane0))
  (AddComponent|AddChildActorComponent false (Math|Transform|MakeTransform (Math|Vector|MakeVector (.x (.location _returnvalue_3)) (.y (.location _returnvalue_3)) (+ (.z (.location _returnvalue_3)) 1.5e+02)) (.rotation _returnvalue_3) (.scale _returnvalue_3)))
  (AddComponent|AddChildActorComponent false (Math|Transform|MakeTransform (Math|Vector|MakeVector (.x (.location _returnvalue_2)) (.y (.location _returnvalue_2)) (+ (.z (.location _returnvalue_2)) 1.5e+02)) (.rotation _returnvalue_2) (.scale _returnvalue_2)))
  (AddComponent|AddChildActorComponent false (Math|Transform|MakeTransform (Math|Vector|MakeVector (.x (.location _returnvalue)) (.y (.location _returnvalue)) (+ (.z (.location _returnvalue)) 1.5e+02)) (.rotation _returnvalue) (.scale _returnvalue))))